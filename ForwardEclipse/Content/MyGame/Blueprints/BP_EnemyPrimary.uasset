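; BP_EnemyPrimary is a Paper2D enemy character that turns toward the player controller's location and fires projectiles.
; Tick checks signed X distance to the player, spawning BP_EnemyProjectile at its arrow, effectively once given a huge DoOnce reset delay.
; EnemyTakesDamage lowers health and, while alive, applies knockback, then raises gravity until landing.
; Health prints every tick; DestroyActor is unconnected, so zero health never removes the enemy.
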(event `EnemyTakesDamage`
  (params (DamageTaken :type "Float (double-precision)") (ForceX :type "Float (double-precision)") (ForceZ :type "Float (double-precision)"))
  ;[1 1 1] Enemy Health (Damage Taken) System
  (bind _output_get (set `self.EnemyCharacterHealth` (- (`self.EnemyCharacterHealth`) DamageTaken)))
  (if (not (<= _output_get 0.0))
    (`CharacterMovementComponent.AddImpulse` (`self.CharacterMovement`) (`KismetMathLibrary.MakeVector` ForceX 0.0 ForceZ) false)
    (`KismetSystemLibrary.RetriggerableDelay` 0.2)
    (set `CharacterMovementComponent.GravityScale` 5.0 (`self.CharacterMovement`))))

(event `self.OnLanded`
  (params (Hit :type "HitResult Structure (by ref)"))
  ;[1 1 1] Enemy Health (Damage Taken) System
  (set `CharacterMovementComponent.GravityScale` 0.0 (`self.CharacterMovement`)))

(event `EnemyFiresProjectile`
  ;[1 1 1] Enemy Projectile System
  (`/Engine/EditorBlueprintResources/StandardMacros.DoOnce` false :!label _label
    (:`Completed`
      (`|SpawnActorFromClass` "/Game/MyGame/Blueprints/BP_EnemyProjectile.BP_EnemyProjectile_C" (`SceneComponent.K2_GetComponentToWorld` (`self.ArrowComponent`)) "AdjustIfPossibleButAlwaysSpawn" "OverrideRootScale")
      (`KismetSystemLibrary.Delay` 100000.0)
      (goto _label :!via `Reset`))))

(event `self.ReceiveTick`
  (params (DeltaSeconds :type "Float (single-precision)"))
  (bind _returnvalue_x (`KismetMathLibrary.BreakVector` (`self.K2_GetActorLocation` (`GameplayStatics.GetPlayerCharacter` 0))))
  (bind _returnvalue_x_2 (`KismetMathLibrary.BreakVector` (`SceneComponent.K2_GetComponentLocation` (`self.PaperSprite`))))
  (bind (_returnvalue_roll _returnvalue_pitch _returnvalue_yaw) (`KismetMathLibrary.BreakRotator` (`KismetMathLibrary.FindLookAtRotation` (`self.K2_GetActorLocation`) (`self.K2_GetActorLocation` (`GameplayStatics.GetPlayerController` 0)))))
  ;[1 1 1] If within range, Fire at character.
  (`|ExecutionSequence`
    (:`then_0`
      (bind _output_get (set `self.Distance` (- _returnvalue_x_2 _returnvalue_x)))
      ;[1 1 1] Enemy Location minus character location
      (if (<= _output_get 250.0)
        (`self.EnemyFiresProjectile`)))
    (:`then_1`
      (`self.K2_SetActorRotation` (`KismetMathLibrary.MakeRotator` 0.0 0.0 _returnvalue_yaw)))
    (:`then_2`
      (`KismetSystemLibrary.PrintString` (`KismetStringLibrary.Conv_DoubleToString` (`self.EnemyCharacterHealth`))))))

(fn `UserConstructionScript`)