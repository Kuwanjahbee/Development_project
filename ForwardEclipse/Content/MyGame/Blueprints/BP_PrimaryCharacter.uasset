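; Player character for a 2D Paper2D side-scrolling auto-runner, pushed forward every Tick, with jump, projectile, melee and uppercut-animated shield inputs.
; Inputs and damage events set CharState, which UpdateAnimation maps to flipbooks.
; BeginPlay creates the HUD and loads weapon row names, which CycleWeapon1 steps through to copy data table stats into variables.
; Melee launches overlapping enemies, while DamageSystem and HealthSystem manage knockback, death and capped healing.
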(event `Weapon_Initialization`
  (bind _outrownames (`DataTableFunctionLibrary.GetDataTableRowNames` null))
  (bind _output_get (set `self.Weapon Array` _outrownames))
  (set `self.Numberofweapons` (`KismetArrayLibrary.Array_Length` _output_get)))

(event `self.ReceiveBeginPlay`
  ;[1 1 1] Begin Play
  (`|ExecutionSequence`
    (:`then_0`
      (bind _returnvalue (`|CreateWidget` "/Game/MyGame/UI/HUD_PrimaryCharacter.HUD_PrimaryCharacter_C" (`GameplayStatics.GetPlayerController` 0)))
      (`UserWidget.AddToViewport` _returnvalue 0))
    (:`then_1`
      (`ActorComponent.SetIsReplicated` (`self.Sprite`) true))
    (:`then_2`
      (`self.Weapon_Initialization`))))

(event `InputAction|CycleWeapon1`
  (params (Key :type "Key Structure" :default "AnyKey"))
  (:`Pressed`
    (bind _output_get (set `self.WeaponIndex` (`KismetMathLibrary.Clamp` (+ (`self.WeaponIndex`) 1) 0 (`self.Numberofweapons`))))
    (bind _returnvalue (`|GetDataTableRow` "/Game/MyGame/Blueprints/WeaponData.WeaponData" (`KismetArrayLibrary.Array_Get` (`self.Weapon Array`) _output_get))
      (:`then`
        (set `self.WeaponName` (break `/Game/MyGame/Blueprints/Struct_Weapons` _returnvalue))
        (set `self.WeaponColor` (`.Color_6_A9F1A3FB441AB6F0891DB69D979E7963` (break `/Game/MyGame/Blueprints/Struct_Weapons` _returnvalue)))
        (set `self.WeaponVelocityX` (`.VelocityX_11_9ADFB3364BC36BE7D7F4A9923EBA1D59` (break `/Game/MyGame/Blueprints/Struct_Weapons` _returnvalue)))
        (set `self.WeaponVelocityZ` (`.VelocityZ_13_5A4F83A5481E6C8FA332FE9A38EF4039` (break `/Game/MyGame/Blueprints/Struct_Weapons` _returnvalue)))
        (set `self.WeaponZRange` (`.VelocityZRAnge_16_83F9864B4C36637CB8B4329D351D9ADB` (break `/Game/MyGame/Blueprints/Struct_Weapons` _returnvalue)))
        (set `self.WeaponScale` (`.Scale_19_5325D2424DF59280BCE68281C8176468` (break `/Game/MyGame/Blueprints/Struct_Weapons` _returnvalue)))
        (set `self.WeaponFlipBook` (`.Flipbook_21_35C16213497F02654B0245829FF10A66` (break `/Game/MyGame/Blueprints/Struct_Weapons` _returnvalue)))))))

(event `self.ReceiveTick`
  (params (DeltaSeconds :type "Float (single-precision)"))
  ;[1 1 1] Tick - Updates animation
  (`self.UpdateAnimation`)
  (`self.AddMovementInput` (`SceneComponent.GetForwardVector` (`self.Sprite`)) 0.5 :!pinned true) ; TODO: Make Scale Force a Variable
  (`/Engine/EditorBlueprintResources/StandardMacros.CompareFloat` (.x (`MovementComponent.Velocity` (`self.GetMovementComponent`)))
    (:`>`
      (`Controller.SetControlRotation` (`self.GetController`) (`KismetMathLibrary.MakeRotator` 0.0 0.0 0.0)))))

(event `UpdateAnimation`
  (bind _sprite (`self.Sprite`))
  (bind _returnvalue (> (`KismetMathLibrary.VSize` (`self.GetVelocity`)) 0.0))
  ;[1 1 1] Handle Animation
  (switch `/Game/MyGame/Blueprints/Enums/EAnimState` (`self.CharState`)
    (:`NewEnumerator0`
      (`PaperFlipbookComponent.SetFlipbook` _sprite (select `bool` _returnvalue :`false` "/Game/MyGame/Flipbooks/A_PrimaryIdle.A_PrimaryIdle" :`true` "/Game/MyGame/Flipbooks/A_PrimaryRun.A_PrimaryRun" :!type "PaperFlipbook Object Reference")))
    (:`NewEnumerator3`
      (`PaperFlipbookComponent.SetFlipbook` _sprite "/Game/MyGame/Flipbooks/A_PrimaryJump.A_PrimaryJump"))
    (:`NewEnumerator4`
      (`PaperFlipbookComponent.SetFlipbook` _sprite (select `bool` _returnvalue :`false` "/Game/MyGame/Flipbooks/A_PrimaryAttack.A_PrimaryAttack" :`true` "/Game/MyGame/Flipbooks/A_PrimaryAttackRun.A_PrimaryAttackRun" :!type "PaperFlipbook Object Reference")))
    (:`NewEnumerator5`
      (`PaperFlipbookComponent.SetFlipbook` _sprite "/Game/MyGame/Flipbooks/A_PrimaryDamaged.A_PrimaryDamaged"))
    (:`NewEnumerator6`
      (`PaperFlipbookComponent.SetFlipbook` _sprite "/Game/MyGame/Flipbooks/A_PrimaryDeath.A_PrimaryDeath"))
    (:`NewEnumerator7`
      (`PaperFlipbookComponent.SetFlipbook` _sprite "/Game/MyGame/Flipbooks/A_PrimaryDiveKick.A_PrimaryDiveKick"))
    (:`NewEnumerator8`
      (`PaperFlipbookComponent.SetFlipbook` _sprite "/Game/MyGame/Flipbooks/A_PrimaryJumpAttack.A_PrimaryJumpAttack"))
    (:`NewEnumerator9`
      (`PaperFlipbookComponent.SetFlipbook` _sprite "/Game/MyGame/Flipbooks/A_PrimarySlide.A_PrimarySlide"))
    (:`NewEnumerator10`
      (`PaperFlipbookComponent.SetFlipbook` _sprite "/Game/MyGame/Flipbooks/A_PrimaryUppercut.A_PrimaryUppercut"))))

(event `InputAction|AttackAction2`
  (params (Key :type "Key Structure" :default "AnyKey"))
  (bind _swordcollision (`self.SwordCollision`))
  (:`Pressed`
    (if (not (`self.UsingAttack2`))
      (set `self.UsingAttack2` true)
      (set `self.CharState` "NewEnumerator7") ; Used for Sword Animation
      (`self.UpdateAnimation`)
      (`KismetSystemLibrary.Delay` 0.2)
      (for _array_element (`PrimitiveComponent.GetOverlappingActors` _swordcollision "/Game/MyGame/Blueprints/BP_EnemyPrimary.BP_EnemyPrimary_C")
        (bind _asbp_enemy_primary (cast `/Game/MyGame/Blueprints/BP_EnemyPrimary` _array_element))
        (if (`PrimitiveComponent.IsOverlappingComponent` _swordcollision (`Character.CapsuleComponent` _asbp_enemy_primary))
          (`/Engine/EditorBlueprintResources/StandardMacros.DoOnce` false :!label _label
            (:`Completed`
              (`KismetSystemLibrary.PrintString` "Damage")
              (`/Game/MyGame/Blueprints/BP_EnemyPrimary.EnemyTakesDamage` _asbp_enemy_primary 0.0 5000000.0 1000000000.0)
              (goto _label :!via `Reset`)))))
      (`KismetSystemLibrary.Delay` 0.2)
      (set `self.UsingAttack2` false)
      (set `self.CharState` "NewEnumerator0"))))

(event `InputAction|AttackAction1`
  (params (Key :type "Key Structure" :default "AnyKey"))
  ;[1 1 1] Handle Projectile Spawn
  (:`Pressed`
    (set `self.CharState` "NewEnumerator4")
    (`|ExecutionSequence`
      (:`then_0`
        (`GameplayStatics.PlaySoundAtLocation` "/Game/MyGame/Sounds/Cue_Fire.Cue_Fire"))
      (:`then_1`
        (`|SpawnActorFromClass` "/Game/MyGame/Blueprints/BP_Projectile.BP_Projectile_C" (`SceneComponent.K2_GetComponentToWorld` (`self.ProjectileSource`)) "AdjustIfPossibleButAlwaysSpawn" "OverrideRootScale")
        (`self.UpdateAnimation` :!label _label_2)
        (`SceneComponent.K2_SetWorldLocation` (`self.WeaponSprite`) (`SceneComponent.GetSocketLocation` (`self.Sprite`) "Socket_0") false false))))
  (:`Released`
    (`KismetSystemLibrary.RetriggerableDelay` 0.35)
    (set `self.CharState` "NewEnumerator0")
    (goto _label_2)))

(event `DamageSystem`
  (params (`Damage In` :type "Float (double-precision)") (ForceX :type "Float (double-precision)") (ForceZ :type "Float (double-precision)"))
  (bind _charactermovement (`self.CharacterMovement`))
  ;[1 1 1] Current Damage System Method
  (set `self.isHit` true)
  (bind _output_get (set `self.HealthCurrent` (- (`self.HealthCurrent`) `Damage In`)))
  (if (<= _output_get 0.0)
    (set `self.CharState` "NewEnumerator6")
    (`CharacterMovementComponent.DisableMovement` _charactermovement)
    (`self.DisableInput` (`GameplayStatics.GetPlayerController` 0))
    (else
      (set `self.CharState` "NewEnumerator5")
      (`CharacterMovementComponent.AddForce` _charactermovement (`KismetMathLibrary.MakeVector` ForceX 0.0 ForceZ))
      (`KismetSystemLibrary.RetriggerableDelay` 0.2)
      (set `self.isHit` false))))

(event `InputAction|AttackAction3`
  (params (Key :type "Key Structure" :default "AnyKey"))
  (:`Pressed`
    (set `self.CharState` "NewEnumerator10") ; Used for Shield Animation
    (`self.UpdateAnimation` :!label _label_3))
  (:`Released`
    (`KismetSystemLibrary.RetriggerableDelay` 0.2)
    (set `self.CharState` "NewEnumerator0")
    (goto _label_3)))

(event `HealthSystem`
  (params (HealthOut :type "Float (double-precision)"))
  ;[1 1 1] Health Pickup/Gain System
  (bind _output_get (set `self.HealthCurrent` (+ HealthOut (`self.HealthCurrent`))))
  (`/Engine/EditorBlueprintResources/StandardMacros.CompareFloat` _output_get 1.0
    (:`>`
      (set `self.HealthCurrent` 1.0))))

(event `InputAction|Jump`
  (params (Key :type "Key Structure" :default "AnyKey"))
  ;[1 1 1] Handle Jump
  (:`Pressed`
    (`self.Jump` :!label _label_4)
    (set `self.CharState` "NewEnumerator3" :!label _label_5))
  (:`Released`
    (`self.StopJumping` :!label _label_6)
    (goto _label_5)))

(event `InputTouch`
  (params (Location :type "Vector Structure") (FingerIndex :type "ETouchIndex Enum"))
  ;[1 1 1] Handle Jump
  (:`Pressed`
    (goto _label_4))
  (:`Released`
    (goto _label_6)))

(event `self.OnLanded`
  (params (Hit :type "HitResult Structure (by ref)"))
  ;[1 1 1] Handle Jump
  (set `self.CharState` "NewEnumerator0")
  (set `self.bisJumping` false))

(fn `UserConstructionScript`)