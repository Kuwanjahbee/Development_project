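; BP_EnemyActor is a 2D Paper sprite enemy that shoots projectiles and can be damaged and destroyed.
; Tick compares signed X positions with the player, firing BP_EnemyProjectile from its Arrow when within the threshold, throttled by a DoOnce and Delay cooldown.
; EnemyTakesDamage subtracts health, destroying the actor at zero or playing a timeline-lerped knockback in a fixed direction, ignoring its force inputs.
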(event `EnemyTakesDamage`
  (params (DamageTaken :type "Float (double-precision)") (ForceX :type "Float (double-precision)") (ForceZ :type "Float (double-precision)"))
  ;[1 1 1] Enemy Health (Damage Taken) System
  (bind _output_get (set `self.EnemyCharacterHealth` (- (`self.EnemyCharacterHealth`) DamageTaken)))
  (if (<= _output_get 0.0)
    (`self.K2_DestroyActor`)
    (else
      (bind (_direction _newtrack_0) (`Timeline|Timeline_0` :!via `PlayFromStart`)
        (:`Update`
          (`self.K2_SetActorLocation` (`KismetMathLibrary.VLerp` (`self.K2_GetActorLocation`) (+ (`self.K2_GetActorLocation`) (10.0 0.0 10.0)) _newtrack_0)))))))

(event `EnemyFiresProjectile`
  ;[1 1 1] Enemy Projectile System
  (`/Engine/EditorBlueprintResources/StandardMacros.DoOnce` false :!label _label
    (:`Completed`
      (`|SpawnActorFromClass` "/Game/MyGame/Blueprints/BP_EnemyProjectile.BP_EnemyProjectile_C" (`SceneComponent.K2_GetComponentToWorld` (`self.Arrow`)) "AdjustIfPossibleButAlwaysSpawn" "OverrideRootScale")
      (`KismetSystemLibrary.Delay` 1.0)
      (goto _label :!via `Reset`))))

(event `self.ReceiveTick`
  (params (DeltaSeconds :type "Float (single-precision)"))
  (bind _returnvalue_x (`KismetMathLibrary.BreakVector` (`self.K2_GetActorLocation` (`GameplayStatics.GetPlayerCharacter` 0))))
  (bind _returnvalue_x_2 (`KismetMathLibrary.BreakVector` (`SceneComponent.K2_GetComponentLocation` (`self.PaperSprite`))))
  ;[1 1 1] If within range, Fire at character.
  (`|ExecutionSequence`
    (:`then_0`
      (bind _output_get (set `self.Distance` (- _returnvalue_x_2 _returnvalue_x)))
      ;[1 1 1] Enemy Location minus character location
      (if (<= _output_get 5.0)
        (`self.EnemyFiresProjectile`)))))

(fn `UserConstructionScript`)