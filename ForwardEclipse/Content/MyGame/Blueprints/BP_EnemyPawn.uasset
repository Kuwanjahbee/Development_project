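; Enemy pawn that shoots projectiles at the player and can be damaged and killed.
; Tick fires when its sprite's X minus the player's X is within a threshold, a signed check that also passes at any distance beyond the enemy in +X.
; A DoOnce reset after a Delay limits projectile spawns at the Arrow to about one per second.
; Damage lowers health, then either destroys the actor or pushes its Sphere with a force.
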(event `EnemyTakesDamage`
  (params (DamageTaken :type "Float (double-precision)") (ForceX :type "Float (double-precision)") (ForceZ :type "Float (double-precision)"))
  ;[1 1 1] Enemy Health (Damage Taken) System
  (bind _output_get (set `self.EnemyCharacterHealth` (- (`self.EnemyCharacterHealth`) DamageTaken)))
  (if (<= _output_get 0.0)
    (`self.K2_DestroyActor`)
    (else
      (`PrimitiveComponent.AddForce` (`self.Sphere`) (`KismetMathLibrary.MakeVector` ForceX 0.0 ForceZ) "None" false))))

(event `EnemyFiresProjectile`
  ;[1 1 1] Enemy Projectile System
  (`/Engine/EditorBlueprintResources/StandardMacros.DoOnce` false :!label _label
    (:`Completed`
      (`|SpawnActorFromClass` "/Game/MyGame/Blueprints/BP_EnemyProjectile.BP_EnemyProjectile_C" (`SceneComponent.K2_GetComponentToWorld` (`self.Arrow`)) "AdjustIfPossibleButAlwaysSpawn" "OverrideRootScale")
      (`KismetSystemLibrary.Delay` 1.0)
      (goto _label :!via `Reset`))))

(event `self.ReceiveTick`
  (params (DeltaSeconds :type "Float (single-precision)"))
  (bind _returnvalue_x (`KismetMathLibrary.BreakVector` (`self.K2_GetActorLocation` (`GameplayStatics.GetPlayerCharacter` 0))))
  (bind _returnvalue_x_2 (`KismetMathLibrary.BreakVector` (`SceneComponent.K2_GetComponentLocation` (`self.PaperSprite`))))
  ;[1 1 1] If within range, Fire at character.
  (if (<= (- _returnvalue_x_2 _returnvalue_x) 400.0)
    (`self.EnemyFiresProjectile`)))

(fn `UserConstructionScript`)